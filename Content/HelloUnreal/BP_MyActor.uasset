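; BP_MyActor is a tutorial-style actor whose static mesh slides back and forth along its local X axis while IsPlay is set.
; Tick steps XPosition one unit per frame and applies it as the mesh's relative X, with IsMoveRight flipping at each end of the range.
; Movement is not scaled by delta time, so speed follows frame rate.
; Disconnected leftover nodes hold a print and an earlier Delay-based stepping sequence.
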(event `self.ReceiveTick`
  (params (DeltaSeconds :type "Float (single-precision)"))
  (if (`self.isPlay`)
    (if (`self.isMoveRight`)
      ;[1 1 1] x+100
      (bind _output_get (set `self.XPosition` (+ (`self.XPosition`) 1.0 0.0)))
      (`SceneComponent.K2_SetRelativeLocation` (`self.StaticMesh`) (`KismetMathLibrary.MakeVector` _output_get) false false)
      (if (>= (`self.XPosition`) 100.0)
        (set `self.isMoveRight` false))
      (else
        ;[1 1 1] x-100
        (bind _output_get_2 (set `self.XPosition` (+ (`self.XPosition`) -1.0 0.0)))
        (`SceneComponent.K2_SetRelativeLocation` (`self.StaticMesh`) (`KismetMathLibrary.MakeVector` _output_get_2) false false)
        (if (< (`self.XPosition`) 0.0)
          (set `self.isMoveRight` true))))))

(fn `UserConstructionScript`)